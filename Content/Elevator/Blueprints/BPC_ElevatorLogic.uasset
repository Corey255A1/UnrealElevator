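; BPC_ElevatorLogic is an actor component that drives its owning elevator upward between stops through a simple state machine.
; Tick moves the owner at constant speed along local Z while Moving, and counts a fixed delay in Pending before switching to Moving.
; Ending overlap with a BP_ElevatorStop sets Pending, while Interact does so only from Complete.
; Every state change broadcasts the new and old states.
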(event `self.ReceiveBeginPlay`
  (add `Actor.OnActorEndOverlap` (`self.GetOwner`) (delegate `OverlappedActor`)))

(event `OverlappedActor`
  (params (OverlappedActor :type "Actor Object Reference") (OtherActor :type "Actor Object Reference"))
  (cast `/Game/Elevator/Blueprints/BP_ElevatorStop` OtherActor)
  (`self.SetElevatorState` "NewEnumerator2"))

(event `self.ReceiveTick`
  (params (DeltaSeconds :type "Float (single-precision)"))
  (`self.DoElevatorLogic` DeltaSeconds))

(event `/Game/Elevator/Blueprints/BPI_Interactable.Interact`
  (params (Player :type "PlayerController Object Reference"))
  (`self.SetPending`))

(fn `DoElevatorLogic`
  (params (`Delta Seconds` :type "Float (double-precision)"))
  (switch `/Game/Elevator/Blueprints/E_ElevatorStates` (`self.CurrentElevatorState`)
    (:`NewEnumerator1`
      (`self.DoMoving` `Delta Seconds`))
    (:`NewEnumerator2`
      (`self.DoPending` `Delta Seconds`))))

(fn `DoMoving`
  (params (`Delta Seconds` :type "Float (double-precision)"))
  (`Actor.K2_AddActorLocalOffset` (`self.GetOwner`) (`KismetMathLibrary.MakeVector` 0.0 0.0 (* `Delta Seconds` 50.0)) false false))

(fn `DoPending`
  (params (`Delta Seconds` :type "Float (double-precision)"))
  (bind _output_get (set `self.CurrentWaitTime` (+ `Delta Seconds` (`self.CurrentWaitTime`))))
  (if (>= _output_get 4.0)
    (`self.SetElevatorState` "NewEnumerator1")
    (set `self.CurrentWaitTime` 0.0)))

(fn `SetElevatorState`
  (params (`New State` :type "/Game/Elevator/Blueprints/E_ElevatorStates Enum" :default "NewEnumerator0"))
  (locals (OldState :type "/Game/Elevator/Blueprints/E_ElevatorStates Enum" :default "NewEnumerator0"))
  (bind _output_get (set `local.OldState` (`self.CurrentElevatorState`)))
  (bind _output_get_2 (set `self.CurrentElevatorState` `New State`))
  (`self.StateChanged` _output_get_2 _output_get))

(fn `SetPending`
  (if (`|EnumEquality` (`self.CurrentElevatorState`) "NewEnumerator0")
    (set `self.CurrentWaitTime` 0.0)
    (`self.SetElevatorState` "NewEnumerator2")))