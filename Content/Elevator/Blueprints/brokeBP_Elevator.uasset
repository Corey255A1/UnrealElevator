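; Elevator actor that moves vertically between floor stops, with a floor panel widget that Activate opens when the elevator is Complete, or closes if already open.
; Tick drives a state machine: Moving offsets the actor along Z by MoveSpeed, and Pending waits four seconds before switching to Moving.
; When ElevatorBase stops overlapping a marked BP_ElevatorStop, it clears the mark and becomes Pending or Complete, depending on remaining marked Floors.
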(event `self.ReceiveTick`
  (params (DeltaSeconds :type "Float (single-precision)"))
  (`self.UpdateElevatorLogic` DeltaSeconds))

(event `/Game/Elevator/Blueprints/BPI_Activateable.Activate`
  (params (Player :type "PlayerController Object Reference"))
  (`self.ToggleMovement` Player))

(event `self.ElevatorBase.OnComponentEndOverlap`
  (params (OverlappedComponent :type "PrimitiveComponent Object Reference") (OtherActor :type "Actor Object Reference") (OtherComp :type "PrimitiveComponent Object Reference") (OtherBodyIndex :type Integer))
  (bind _asbp_elevator_stop (cast `/Game/Elevator/Blueprints/BP_ElevatorStop` OtherActor))
  (`self.ProcessElevatorStop` _asbp_elevator_stop))

(fn `AreThereMoreStops`
  (returns (AreMoreStops :type Boolean))
  (locals (FoundStop :type Boolean))
  (for _array_element (`self.Floors`)
    (if (`/Game/Elevator/Blueprints/BP_ElevatorStop.IsMarkedForStop` _array_element)
      (set `local.FoundStop` true)
      (break)))
  (return (`local.FoundStop`)))

(fn `MovingState`
  (params (`Delta Seconds` :type "Float (double-precision)"))
  (`self.K2_AddActorLocalOffset` (`KismetMathLibrary.MakeVector` 0.0 0.0 (* `Delta Seconds` (`self.MoveSpeed`)))))

(fn `PendingState`
  (params (DeltaSeconds :type "Float (double-precision)"))
  (bind _output_get (set `self.WaitTime` (+ DeltaSeconds (`self.WaitTime`))))
  (if (>= _output_get 4.0)
    (`self.SetElevatorState` "NewEnumerator1")
    (set `self.WaitTime` 0.0)))

(fn `ProcessElevatorStop`
  (params (ElevatorStop :type "/Game/Elevator/Blueprints/BP_ElevatorStop Object Reference"))
  (if (`/Game/Elevator/Blueprints/BP_ElevatorStop.IsMarkedForStop` ElevatorStop)
    (set `/Game/Elevator/Blueprints/BP_ElevatorStop.IsMarkedForStop` false ElevatorStop)
    (bind _aremorestops (`self.AreThereMoreStops`))
    (if _aremorestops
      (`self.SetElevatorState` "NewEnumerator2")
      (else
        (`self.SetElevatorState` "NewEnumerator0")))))

(fn `SetElevatorState`
  (params (NextState :type "/Game/Elevator/Blueprints/E_ElevatorStates Enum" :default "NewEnumerator0"))
  (bind _output_get (set `self.State` NextState))
  (`self.StateChanged` _output_get NextState))

(fn `ToggleMovement`
  (params (Player :type "PlayerController Object Reference"))
  (locals (Owner :type "PlayerController Object Reference"))
  (set `local.Owner` Player)
  (`/Engine/EditorBlueprintResources/StandardMacros.IsValid` (`self.CurrentFloorMenu`)
    (:`Is Valid`
      (`Widget.RemoveFromParent` (`self.CurrentFloorMenu`))
      (set `self.CurrentFloorMenu` null)
      (set `PlayerController.bShowMouseCursor` false))
    (:`Is Not Valid`
      (switch `/Game/Elevator/Blueprints/E_ElevatorStates` (`self.State`)
        (:`NewEnumerator0`
          (bind _returnvalue (`|CreateWidget` "/Game/Elevator/Blueprints/BPW_ElevatorPanel.BPW_ElevatorPanel_C"))
          (bind _output_get (set `self.CurrentFloorMenu` _returnvalue))
          (`UserWidget.AddToViewport` _output_get 0)
          (`WidgetBlueprintLibrary.SetInputMode_GameAndUIEx` null (`self.CurrentFloorMenu`))
          (set `PlayerController.bShowMouseCursor` true))))))

(fn `UpdateElevatorLogic`
  (params (DeltaSeconds :type "Float (double-precision)"))
  (switch `/Game/Elevator/Blueprints/E_ElevatorStates` (`self.State`)
    (:`NewEnumerator1`
      (`self.MovingState` DeltaSeconds))
    (:`NewEnumerator2`
      (`self.PendingState` DeltaSeconds))))

(fn `UserConstructionScript`)